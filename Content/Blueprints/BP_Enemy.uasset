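; Golem enemy actor that takes damage and dies, with fire or ice plane and health bar materials set by Type at construction.
; Until dying, Tick eases the Cube's Z scale toward 1, passing game time rather than frame delta to FInterpTo.
; TakeDamage lowers HP and rescales the bar; its death check subtracts Value again.
; Death plays the ActorSequence and a camera shake, then destroys the actor on a timer.
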(event `self.ReceiveBeginPlay`
  (bind _returnvalue (`KismetMathLibrary.FInterpTo` 0.0 3.0 (`GameplayStatics.GetTimeSeconds`) 0.5))
  (`SceneComponent.SetRelativeScale3D` (`self.Cube`) (`KismetMathLibrary.MakeVector` _returnvalue _returnvalue _returnvalue)))

(event `self.ReceiveTick`
  (params (DeltaSeconds :type "Float (single-precision)"))
  (if (not (`self.Dying`))
    (bind _output_get (set `self.ScaleInterpCurrent` (`KismetMathLibrary.FInterpTo` (`self.ScaleInterpCurrent`) 1.0 (`GameplayStatics.GetTimeSeconds`) 0.1)))
    (`SceneComponent.SetRelativeScale3D` (`self.Cube`) (`KismetMathLibrary.MakeVector` 10.0 3.0 _output_get))))

(fn `Die`
  (`self.K2_DestroyActor`))

(fn `TakeDamage`
  (params (Value :type "Float (double-precision)"))
  (bind _returnvalue (- (`self.HP`) Value))
  (bind _output_get (set `self.HP` _returnvalue))
  (`SceneComponent.SetRelativeScale3D` (`self.HealthBar`) (`KismetMathLibrary.MakeVector` (/ _output_get 100.0)))
  (if (<= _returnvalue 0.0)
    (set `self.Dying` true)
    (`MovieSceneSequencePlayer.Play` (`ActorSequenceComponent.SequencePlayer` (`self.ActorSequence`)))
    (`KismetSystemLibrary.K2_SetTimer` null "Die" 1.0)
    (`MatineeCameraShake.StartMatineeCameraShake` (`GameplayStatics.GetPlayerCameraManager` 0) "/Game/Blueprints/BP_CameraSHake.BP_CameraShake_C" 1.0 "World")))

(fn `UserConstructionScript`
  (bind _plane (`self.Plane`))
  (bind _healthbar (`self.HealthBar`))
  (if (`|EnumEquality` (`self.Type`) "NewEnumerator0")
    (`PrimitiveComponent.SetMaterial` _plane 0 "/Game/Textures/Fire_golem_Mat.Fire_golem_Mat")
    (`PrimitiveComponent.SetMaterial` _healthbar 0 "/Game/Materials/M_EmissiveHot.M_EmissiveHot")
    (else
      (`PrimitiveComponent.SetMaterial` _plane 0 "/Game/Textures/Ice_golem_Mat.Ice_golem_Mat")
      (`PrimitiveComponent.SetMaterial` _healthbar 0 "/Game/Materials/M_EmissiveCold.M_EmissiveCold"))))