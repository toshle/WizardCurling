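; BP_LevelTile is a moving level tile that spawns its own successor to form an endless scrolling level.
; Tick slides it along its local negative Y axis by a fixed, frame-rate-dependent step.
; The first BP_Wizard overlap with its Box spawns another scaled, rotated tile at a fixed world X offset, guarded by a Spawned flag.
; Each tile destroys itself one minute after BeginPlay.
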(event `self.ReceiveBeginPlay`
  (`KismetSystemLibrary.Delay` 60.0)
  (`self.K2_DestroyActor`))

(event `self.ReceiveTick`
  (params (DeltaSeconds :type "Float (single-precision)"))
  (`SceneComponent.K2_AddLocalOffset` (`self.DefaultSceneRoot`) (0.0 -10.0 0.0) false true))

(event `self.Box.OnComponentBeginOverlap`
  (params (OverlappedComponent :type "PrimitiveComponent Object Reference") (OtherActor :type "Actor Object Reference") (OtherComp :type "PrimitiveComponent Object Reference") (OtherBodyIndex :type Integer) (bFromSweep :type Boolean) (SweepResult :type "HitResult Structure (by ref)"))
  (bind (_returnvalue_x _returnvalue_y _returnvalue_z) (`KismetMathLibrary.BreakVector` (`SceneComponent.K2_GetComponentLocation` (`self.DefaultSceneRoot`))))
  (cast `/Game/Blueprints/BP_Wizard` OtherActor)
  (if (not (`self.Spawned`))
    (set `self.Spawned` true)
    (`|SpawnActorFromClass` "BP_LevelTile_C" (`KismetMathLibrary.MakeTransform` (`KismetMathLibrary.MakeVector` (+ _returnvalue_x -19000.0) _returnvalue_y _returnvalue_z) (struct :`Yaw` 90.0) (2.0 2.0 2.0)) "Undefined" "OverrideRootScale" null null)
    (`KismetSystemLibrary.PrintString` "Next Tile" true true (struct :`R` 1.0 :`B` 0.795874 :`A` 1.0))))

(fn `UserConstructionScript`)