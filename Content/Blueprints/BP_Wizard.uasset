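; Player wizard that catches fire and ice projectiles to build elemental energy and score, then spends it on attacks.
; Mouse axis input slides the Fire and Ice components in opposite directions, while movement axes offset the Texture component.
; Sphere overlaps destroy matching projectiles and charge that element, with energy pushed to the HUD every tick.
; Attack inputs spawn a fireball or ice bolt at full charge and reset that energy.
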(event `InputAxis|MouseRotation`
  (params (AxisValue :type "Float (single-precision)"))
  (bind _fire (`self.Fire`))
  (bind _returnvalue (* AxisValue (`self.ExpandRate`)))
  (bind (_relativelocation_x _relativelocation_y) (`KismetMathLibrary.BreakVector` (`SceneComponent.RelativeLocation` _fire)))
  (if (> _relativelocation_y 1500.0)
    (`SceneComponent.K2_AddRelativeLocation` _fire (`KismetMathLibrary.MakeVector` 0.0 _returnvalue) true false :!label _label)
    (`SceneComponent.K2_AddRelativeLocation` (`self.Ice`) (`KismetMathLibrary.MakeVector` 0.0 (* _returnvalue -1.0)) true false)
    (elif (!= AxisValue 0.0)
      (goto _label))))

(event `self.IceSphere.OnComponentBeginOverlap`
  (params (OverlappedComponent :type "PrimitiveComponent Object Reference") (OtherActor :type "Actor Object Reference") (OtherComp :type "PrimitiveComponent Object Reference") (OtherBodyIndex :type Integer) (bFromSweep :type Boolean) (SweepResult :type "HitResult Structure (by ref)"))
  (bind _asbp_ice_projectile (cast `/Game/Blueprints/BP_IceProjectile` OtherActor))
  (`self.K2_DestroyActor` _asbp_ice_projectile)
  (set `self.IceEnergy` (+ (`self.IceEnergy`) 0.5))
  (`KismetSystemLibrary.PrintString` "Ice")
  (bind _output_get (set `self.Score` (+ (`self.Score`) 10.0) :!label _label_2))
  (`/Game/GUI/WBP_HUD.UpdateScore` (stale `self.ReceiveBeginPlay` _returnvalue) _output_get))

(event `self.FireSphere.OnComponentBeginOverlap`
  (params (OverlappedComponent :type "PrimitiveComponent Object Reference") (OtherActor :type "Actor Object Reference") (OtherComp :type "PrimitiveComponent Object Reference") (OtherBodyIndex :type Integer) (bFromSweep :type Boolean) (SweepResult :type "HitResult Structure (by ref)"))
  (bind _asbp_fire_projectile (cast `/Game/Blueprints/BP_FireProjectile` OtherActor))
  (`self.K2_DestroyActor` _asbp_fire_projectile)
  (set `self.FireEnergy` (+ (`self.FireEnergy`) 0.5))
  (`KismetSystemLibrary.PrintString` "Fire" true true (struct :`R` 1.0 :`G` 0.097106 :`A` 1.0))
  (goto _label_2))

(event `self.ReceiveTick`
  (params (DeltaSeconds :type "Float (single-precision)"))
  (`/Game/GUI/WBP_HUD.UpdateEnergies` (stale `self.ReceiveBeginPlay` _returnvalue) (`self.FireEnergy`) (`self.IceEnergy`) false))

(event `self.ReceiveBeginPlay`
  (bind _returnvalue (`|CreateWidget` "/Game/GUI/WBP_HUD.WBP_HUD_C"))
  (`UserWidget.AddToViewport` _returnvalue 0))

(event `InputAction|FireAttack`
  (params (Key :type "Key Structure"))
  (:`Pressed`
    (if (>= (`self.FireEnergy`) 100.0)
      (`|SpawnActorFromClass` "/Game/Blueprints/BP_FireBall.BP_FireBall_C" (`KismetMathLibrary.MakeTransform` (`SceneComponent.K2_GetComponentLocation` (`self.FireAttackArrow`)) (struct :`Yaw` 180.0) (3.0 3.0 3.0)) "Undefined" "OverrideRootScale" null null)
      (set `self.FireEnergy` 0.0))))

(event `InputAction|IceAttack`
  (params (Key :type "Key Structure"))
  (:`Pressed`
    (if (>= (`self.IceEnergy`) 100.0)
      (`|SpawnActorFromClass` "/Game/Blueprints/BP_IceBolt.BP_IceBolt_C" (`KismetMathLibrary.MakeTransform` (`SceneComponent.K2_GetComponentLocation` (`self.IceAttackArrow`)) (struct :`Yaw` 180.0) (3.0 3.0 3.0)) "Undefined" "OverrideRootScale" null null)
      (set `self.IceEnergy` 0.0))))

(event `InputAxis|MoveRight`
  (params (AxisValue :type "Float (single-precision)"))
  (bind _texture (`self.Texture`))
  (bind (_relativelocation_x _relativelocation_y _relativelocation_z) (`KismetMathLibrary.BreakVector` (`SceneComponent.RelativeLocation` _texture)))
  (`SceneComponent.K2_SetRelativeLocation` _texture (`KismetMathLibrary.MakeVector` _relativelocation_x (* (`self.StepSize`) AxisValue) _relativelocation_z) false false))

(event `InputAxis|MoveForward`
  (params (AxisValue :type "Float (single-precision)"))
  (bind _texture (`self.Texture`))
  (bind (_relativelocation_x _relativelocation_y _relativelocation_z) (`KismetMathLibrary.BreakVector` (`SceneComponent.RelativeLocation` _texture)))
  (`SceneComponent.K2_SetRelativeLocation` _texture (`KismetMathLibrary.MakeVector` (* (`self.StepSize`) AxisValue) _relativelocation_y _relativelocation_z) false false))

(fn `UserConstructionScript`)