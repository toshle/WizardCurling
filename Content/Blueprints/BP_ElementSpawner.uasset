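; BP_ElementSpawner plays a sound and spawns fire and ice projectiles in response to its loudness.
; On BeginPlay it binds to the audio component's playback percent event, which triggers both spawns on every update.
; Playback percent times duration gives the time to sample channel 0 in LoudnessRef.
; That loudness plus the arrow's Y is scaled and offset in opposite directions, placing fire and ice on mirrored Y positions.
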(event `self.ReceiveBeginPlay`
  (bind _sound (`self.Sound`))
  (bind _audio (`self.Audio`))
  (`AudioComponent.SetSound` (`self.Audio`) _sound)
  (set `self.Duration` (`SoundBase.Duration` _sound))
  (add `AudioComponent.OnAudioPlaybackPercent` _audio (delegate `PlaybackChange`))
  (`AudioComponent.Play` _audio 0.0))

(event `PlaybackChange`
  (params (PlayingSoundWave :type "SoundWave Object Reference") (PlaybackPercent :type "Float (double-precision)"))
  (`self.SpawnFire` PlaybackPercent)
  (`self.SpawnIce` PlaybackPercent))

(fn `SpawnFire`
  (params (PlaybackPercent :type "Float (double-precision)"))
  (bind (_returnvalue_x _returnvalue_y _returnvalue_z) (`KismetMathLibrary.BreakVector` (`SceneComponent.K2_GetComponentLocation` (`self.Arrow`))))
  (bind _output_get (set `self.PlayTime` (* PlaybackPercent (`self.Duration`))))
  (`|SpawnActorFromClass` "/Game/Blueprints/BP_FireProjectile.BP_FireProjectile_C" (`KismetMathLibrary.MakeTransform` (`KismetMathLibrary.MakeVector` _returnvalue_x (+ (* 200 (+ (`LoudnessNRT.GetChannelLoudnessAtTime` (`self.LoudnessRef`) _output_get 0) _returnvalue_y)) 2000.0) _returnvalue_z)) "Undefined" "OverrideRootScale" null null))

(fn `SpawnIce`
  (params (PlaybackPercent :type "Float (double-precision)"))
  (bind (_returnvalue_x _returnvalue_y _returnvalue_z) (`KismetMathLibrary.BreakVector` (`SceneComponent.K2_GetComponentLocation` (`self.Arrow`))))
  (bind _output_get (set `self.PlayTime` (* PlaybackPercent (`self.Duration`))))
  (`|SpawnActorFromClass` "/Game/Blueprints/BP_IceProjectile.BP_IceProjectile_C" (`KismetMathLibrary.MakeTransform` (`KismetMathLibrary.MakeVector` _returnvalue_x (+ (* -200 (+ (`LoudnessNRT.GetChannelLoudnessAtTime` (`self.LoudnessRef`) _output_get 0) _returnvalue_y)) -2000.0) _returnvalue_z)) "Undefined" "OverrideRootScale" null null))

(fn `UserConstructionScript`)